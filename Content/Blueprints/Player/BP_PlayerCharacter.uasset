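; Player character Blueprint with forward-axis movement and a held slow-motion input.
; BeginPlay adds the player input mapping context and fills the slow-mo charge.
; Holding slow-mo lowers a target time scale that Tick eases toward, and the result scales only the character's movement input, leaving global time dilation untouched.
; Charge drops by one frame's delta when movement starts, but never gates slow motion.
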(event `self.ReceiveBeginPlay`
  (bind _asbp_player_controller (cast `/Game/Blueprints/Player/BP_PlayerController` (`GameplayStatics.GetPlayerController` 0))
    (:`then`
      (`EnhancedInputSubsystemInterface.AddMappingContext` (pcsubsystem `EnhancedInputLocalPlayerSubsystem` _asbp_player_controller) "/Game/Blueprints/Input/IMC_PlayerController.IMC_PlayerController" 0 (struct))
      (set `self.CurrentSlowMoCharge` (`self.MaxSloMoCharge`)))
    (:`CastFailed`
      (`KismetSystemLibrary.PrintString` "Cast Failed"))))

(event `EnhancedInput|/Game/Blueprints/Input/IA_Move`
  (params (ActionValue :type "Float (double-precision)") (ElapsedSeconds :type "Float (double-precision)") (TriggeredSeconds :type "Float (double-precision)") (InputAction :type "InputAction Object Reference" :default "/Game/Blueprints/Input/IA_Move.IA_Move"))
  (:`Triggered`
    (`self.AddMovementInput` (`self.GetActorForwardVector`) (* ActionValue (`self.TimeScale`))))
  (:`Started`
    (set `self.CurrentSlowMoCharge` (- (`self.CurrentSlowMoCharge`) (`self.Delta Seconds`)))))

(event `self.ReceiveTick`
  (params (DeltaSeconds :type "Float (single-precision)"))
  (set `self.Delta Seconds` DeltaSeconds)
  (set `self.TimeScale` (`|EaseFunction` "Linear" 0.1 (`self.TimeScale`) (`self.TargetTimeScale`))))

(event `EnhancedInput|/Game/Blueprints/Input/IA_SloMo`
  (params (ActionValue :type Boolean) (ElapsedSeconds :type "Float (double-precision)") (TriggeredSeconds :type "Float (double-precision)") (InputAction :type "InputAction Object Reference" :default "/Game/Blueprints/Input/IA_SloMo.IA_SloMo"))
  (:`Started`
    (set `self.TargetTimeScale` 0.3))
  (:`Completed`
    (set `self.TargetTimeScale` 1.0)))

(fn `UserConstructionScript`)